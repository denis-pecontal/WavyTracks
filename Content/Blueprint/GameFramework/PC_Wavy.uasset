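; PC_Wavy is a player controller that handles pausing and the pause menu.
; On BeginPlay it creates the Pause widget, adds it hidden to the viewport and sets game-only input.
; The Pause input action pauses the game and shows the menu and mouse cursor, leaving the input mode unchanged.
; The Unpause event reverses this, with no caller in this graph.
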(event `self.ReceiveBeginPlay`
  (bind _returnvalue (`|CreateWidget` "/Game/HUD/Pause.Pause_C" self))
  (bind _output_get (set `self.pauseMenu` _returnvalue))
  (`UserWidget.AddToViewport` _output_get 0)
  (`Widget.SetVisibility` _output_get "Hidden")
  (`WidgetBlueprintLibrary.SetInputMode_GameOnly` self))

(event `InputAction|Pause`
  (params (Key :type "Key Structure"))
  (:`Pressed`
    (`GameplayStatics.SetGamePaused` true)
    (`Widget.SetVisibility` (`self.pauseMenu`) "Visible")
    (set `self.bShowMouseCursor` true)))

(event `Unpause`
  (`GameplayStatics.SetGamePaused` false)
  (`Widget.SetVisibility` (`self.pauseMenu`) "Hidden")
  (set `self.bShowMouseCursor` false))

(fn `UserConstructionScript`)