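; GM_Track is the game mode for a track level that can be opened in Game or Edit mode.
; On BeginPlay it parses the "mode" travel option, printing the active mode for those two values and opening the Menu level otherwise.
; It exposes events to raise a clamped score multiplier or reset it to zero, while the score increment event is an empty stub.
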(event `self.ReceiveBeginPlay`
  (switch `string` (`GameplayStatics.ParseOption` (`self.OptionsString`) "mode")
    (:`Default`
      (`GameplayStatics.OpenLevel` "Menu"))
    (:`game`
      (`KismetSystemLibrary.PrintString` "Game mode" true true (struct :`R` 0.126998 :`G` 1.0 :`A` 1.0) 40.0))
    (:`edit`
      (`KismetSystemLibrary.PrintString` "Edit mode" true true (struct :`R` 0.324347 :`G` 1.0 :`A` 1.0) 40.0))))

(event `IncrementMultiplier`
  (set `self.multiplier` (`KismetMathLibrary.Clamp` (+ (`self.multiplier`) 1) 1 8)))

(event `ResetMultiplier`
  (set `self.multiplier` 0))

(event `IncrementScore`
  (params (Points :type Integer)))

(fn `UserConstructionScript`)